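; Follower is an actor that drifts between the first PillarFollowerSpawn in the level and a PersonID target, based on a Reached flag.
; Each tick it eases its location with VInterpTo toward PersonID while Reached is set, clearing the flag when close, and otherwise toward the pillar.
; The proximity check that would set Reached at the pillar is disconnected, so this graph never sends it back to the person.
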(event `self.ReceiveBeginPlay`
  (bind _outactors (`GameplayStatics.GetAllActorsOfClass` "/Game/Blueprints/PillarFollowerSpawn.PillarFollowerSpawn_C"))
  (set `self.Pillar` (`|GetArrayItem` _outactors)))

(event `self.ReceiveTick`
  (params (DeltaSeconds :type "Float (single-precision)"))
  ;[0.1021 0 1] Sphere<->Character&&Sphere<->Character
  (if (`self.reached`)
    (`self.K2_SetActorLocation` (`KismetMathLibrary.VInterpTo` (`self.K2_GetActorLocation`) (`self.K2_GetActorLocation` (`self.PersonID`)) DeltaSeconds 1.0))
    (if (< (`KismetMathLibrary.Vector_Distance` (`self.K2_GetActorLocation` (`self.PersonID`)) (`self.K2_GetActorLocation`)) 100.0)
      (set `self.reached` false))
    (else
      (`self.K2_SetActorLocation` (`KismetMathLibrary.VInterpTo` (`self.K2_GetActorLocation`) (`self.K2_GetActorLocation` (`self.Pillar`)) DeltaSeconds 1.0)))))

(fn `UserConstructionScript`)